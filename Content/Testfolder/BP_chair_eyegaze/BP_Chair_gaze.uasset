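; Chair actor from an eye-gaze test folder that keeps its WindowPosition component turned toward the player's camera.
; Each tick it casts player character 0 to BP_Pawn_Base and computes a look-at rotation from WindowPosition to that camera.
; RInterpTo eases the component's world rotation toward that target, so it follows smoothly instead of snapping.
; The graph contains no gaze detection, and its CompWindowSimple references are unused.
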(event EventBeginPlay
  (|CallParentFunction))

(event Collision|EventActorBeginOverlap
  (params (OtherActor :type Actor%20Object%20Reference))
  (|CallParentFunction OtherActor) ; This node is disabled and will not be called.\nDrag off pins to build functionality.
)

(event EventTick
  (params (DeltaSeconds :type Float%20%28single-precision%29))
  (bind _windowposition (Variables|Default|GetWindowPosition))
  (|CallParentFunction DeltaSeconds)
  (bind _asbp_pawn_base (Utilities|Casting|CastToBP_Pawn_Base (Game|GetPlayerCharacter 0)))
  (Transformation|SetWorldRotation (Variables|Default|GetWindowPosition) (Math|Interpolation|RInterpTo (Transformation|GetWorldRotation _windowposition) (Math|Rotator|FindLookatRotation (Transformation|GetWorldLocation _windowposition) (Transformation|GetWorldLocation (Default|GetCameraComponent _asbp_pawn_base))) (Utilities|Time|GetWorldDeltaSeconds) 5.0) false false))

(fn ConstructionScript
  (|CallParentFunction))