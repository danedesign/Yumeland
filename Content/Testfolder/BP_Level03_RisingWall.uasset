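; Level 03 actor with four walls that rise in response to velocity changes.
; Each Comp_Velocity change moves the front, left, back and right walls along local Z at progressively smaller fractions of the velocity.
; Tick waits for the front wall to reach a height threshold, then steps the others up each frame to match it.
; When the right wall catches up, it sets Spawncheck.
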(event VelocityChanged(Comp_Velocity)
  (params (SourceInfo :type Struct%20Component%20Source%20Info%20Structure) (Value :type Struct%20Velocity%20Structure))
  (bind _frontwall (Variables|Default|GetFrontWall))
  (bind _leftwall (Variables|Default|GetLeftWall))
  (bind _backwall (Variables|Default|GetBackWall))
  (bind _rightwall (Variables|Default|GetRightWall))
  (Utilities|FlowControl|Sequence
    (:then_0
      ;[1 1 1] Frontwall
      (bind _output_get (Variables|Default|SetPublic_Value_Velocity_Rate (* (.velocity Value) 0.2)))
      (Class|SceneComponent|AddLocalTransform _frontwall (Math|Transform|MakeTransform (Math|Vector|MakeVector 0.0 0.0 _output_get) "0, 0, 0" (Transformation|GetWorldScale _frontwall)) false false))
    (:then_1
      ;[1 1 1] Leftwall
      (Class|SceneComponent|AddLocalTransform _leftwall (Math|Transform|MakeTransform (Math|Vector|MakeVector 0.0 0.0 (* (.velocity Value) 0.18)) "0, 0, 0" (Transformation|GetWorldScale _leftwall)) false false))
    (:then_2
      ;[1 1 1] Backwall
      (Class|SceneComponent|AddLocalTransform _backwall (Math|Transform|MakeTransform (Math|Vector|MakeVector 0.0 0.0 (* (.velocity Value) 0.16)) "0, 0, 0" (Transformation|GetWorldScale _backwall)) false false))
    (:then_3
      ;[1 1 1] Rightwall
      (Class|SceneComponent|AddLocalTransform _rightwall (Math|Transform|MakeTransform (Math|Vector|MakeVector 0.0 0.0 (* (.velocity Value) 0.14)) "0, 0, 0" (Transformation|GetWorldScale _rightwall)) false false))))

(event Collision|EventActorBeginOverlap
  (params (OtherActor :type Actor%20Object%20Reference)))

(event EventTick
  (params (DeltaSeconds :type Float%20%28single-precision%29))
  (bind _leftwall (Variables|Default|GetLeftWall))
  (bind _backwall (Variables|Default|GetBackWall))
  (bind _rightwall (Variables|Default|GetRightWall))
  (bind _returnvalue (Transformation|GetWorldLocation _rightwall))
  (bind _returnvalue_2 (Transformation|GetWorldLocation _leftwall))
  (bind _returnvalue_3 (Transformation|GetWorldLocation _backwall))
  ;[1 1 1] Check if first wall reach the highest?
  (if (>= (.z (Transformation|GetWorldLocation (Variables|Default|GetFrontWall))) 449.0)
    (Utilities|FlowControl|Sequence
      (:then_0
        ;[1 1 1] Check if L Z value equals F Z value
        (if (not (>= (.z (Transformation|GetWorldLocation (Variables|Default|GetLeftWall))) (.z (Transformation|GetWorldLocation (Variables|Default|GetFrontWall)))))
          ;[1 1 1] Add world location to L Z value
          (Transformation|SetWorldLocation _leftwall (Math|Vector|MakeVector (.x _returnvalue_2) (.y _returnvalue_2) (+ (.z _returnvalue_2) 1.0)) false false)))
      (:then_1
        ;[1 1 1] Check if B Z value equals F Z value
        (if (not (>= (.z (Transformation|GetWorldLocation (Variables|Default|GetBackWall))) (.z (Transformation|GetWorldLocation (Variables|Default|GetFrontWall)))))
          ;[1 1 1] Add world location to B Z value
          (Transformation|SetWorldLocation _backwall (Math|Vector|MakeVector (.x _returnvalue_3) (.y _returnvalue_3) (+ (.z _returnvalue_3) 1.0)) false false)))
      (:then_2
        ;[1 1 1] Check if R Z value equals F Z value
        (if (not (>= (.z (Transformation|GetWorldLocation (Variables|Default|GetRightWall))) (.z (Transformation|GetWorldLocation (Variables|Default|GetFrontWall)))))
          ;[1 1 1] Add world location to R Z value
          (Transformation|SetWorldLocation _rightwall (Math|Vector|MakeVector (.x _returnvalue) (.y _returnvalue) (+ (.z _returnvalue) 1.0)) false false)
          ;[1 1 1] Check if R Z value equals F Z value
          (if (>= (.z (Transformation|GetWorldLocation (Variables|Default|GetRightWall))) (.z (Transformation|GetWorldLocation (Variables|Default|GetFrontWall))))
            (Variables|Default|Setspawncheck? true)
            ;[1 1 1] optimization
            (Utilities|FlowControl|Delay 0.5)))))))

(fn ConstructionScript)