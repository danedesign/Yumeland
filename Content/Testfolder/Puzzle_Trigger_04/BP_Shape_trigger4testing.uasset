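; BP_Shape_trigger4testing is a test shape for puzzle trigger 04 whose static mesh follows a slider pole's height.
; BeginPlay keeps the mesh's X and Y and sets its Z from a stored trigger-location variable, whose name marks it as needing a fix.
; Each Tick searches for all BP_SliderPole_Physic_trigger_04 actors and copies the first one's Transformdata Z when its Tag matches RecepterTag.
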(event EventBeginPlay
  (bind _staticmesh (Variables|Default|GetStaticMesh))
  (bind _returnvalue (Transformation|GetWorldLocation _staticmesh))
  (Transformation|SetWorldLocation _staticmesh (Math|Vector|MakeVector (.x _returnvalue) (.y _returnvalue) (Variables|Default|GetSlidepole_trigger_Locationdata%20%28socket%20in%20moddle%29%20needtobefixed)) false false))

(event EventTick
  (params (DeltaSeconds :type Float%20%28single-precision%29))
  (bind _staticmesh (Variables|Default|GetStaticMesh))
  (bind _returnvalue (Transformation|GetWorldLocation _staticmesh))
  (bind _outactors (Actor|GetAllActorsOfClass "/Game/Testfolder/Puzzle_Trigger_04/BP_SliderPole_Physic_trigger_04.BP_SliderPole_Physic_trigger_04_C"))
  (if (Utilities|Enum|Equal(Enum) (Variables|Default|Getrecepter_tag) (Variables|/Game/Testfolder/Puzzle_Trigger_04/BP_SliderPole_Physic_trigger_04.BP_SliderPole_Physic_trigger_04_C|Gettag (Utilities|Array|Get(acopy) _outactors)))
    (Transformation|SetWorldLocation _staticmesh (Math|Vector|MakeVector (.x _returnvalue) (.y _returnvalue) (.z (.location (Variables|/Game/Testfolder/Puzzle_Trigger_04/BP_SliderPole_Physic_trigger_04.BP_SliderPole_Physic_trigger_04_C|Gettransformdata (Utilities|Array|Get(acopy) _outactors))))) false false)))

(fn ConstructionScript
  (|CallParentFunction))