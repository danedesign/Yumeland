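; VR bow that draws with the motion controller trigger and fires attached projectiles on release.
; Trigger pull is stored, drives the skeletal mesh's Extend animation value and scales haptics on the holding controller.
; When the latch releases with draw above a threshold, each attached actor is detached and shot using the pull percentage.
; Attach events disable collision on attached actors and restore it on detach.
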(event ActorLatchReleased(Comp_Latch)
  (if (> (Variables|Default|GetProcent) 0.4)
    (for _array_element (Variables|Default|GetAttachedActorSet (Variables|Default|GetComp_Attach))
      (bind _asbp_arrow (Utilities|Casting|CastTo _array_element))
      ;[1 1 1] This actually makes sense!
      (CallFunction|Detach (Variables|Default|GetComp_Grab _asbp_arrow))
      (CallFunction|Shoot _asbp_arrow (stale TriggerConstant(Comp_ListenToTrigger) Percent)))))

(event TriggerConstant(Comp_ListenToTrigger)
  (params (Percent :type Float%20%28single-precision%29))
  (Variables|Default|SetProcent Percent)
  (bind _asanim_bp_long_bow (Utilities|Casting|CastTo (Components|SkeletalMesh|GetAnimInstance (Variables|Default|GetSkeletalMesh)))
    (:then
      (Variables|Default|SetExtend _asanim_bp_long_bow Percent))
    (:CastFailed
      _))
  (bind _asbp_mcomp (Utilities|Casting|CastTo (Actor|GetAttachParentActor)))
  (CallFunction|SetHaptics :MotionController (Variables|Default|GetBaseMotionController _asbp_mcomp) :Haptics 0 :Curve 0 :Duration 0.1 :Strength (* Percent 5.0)))

(event ActorAttached(Comp_Attach)
  (params (NewlyAttachedActor :type Actor%20Object%20Reference))
  (Collision|SetActorEnableCollision NewlyAttachedActor false))

(event ActorDetached(Comp_Attach)
  (params (DetachedActor :type Actor%20Object%20Reference))
  (Collision|SetActorEnableCollision DetachedActor true))

(event EventBeginPlay)

(event Collision|EventActorBeginOverlap
  (params (OtherActor :type Actor%20Object%20Reference)))

(event EventTick
  (params (DeltaSeconds :type Float%20%28single-precision%29)))

(fn ConstructionScript)