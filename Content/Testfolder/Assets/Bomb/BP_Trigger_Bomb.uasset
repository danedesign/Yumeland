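; BP_Trigger_Bomb is a countdown bomb actor controlled by start and stop triggers received through Comp_Trigger.
; Start shows the remaining time on a TextRender and runs a looping one-second timer, while Stop pauses that timer.
; At zero, a timeline scales and lowers the bomb mesh, and its Explode event spawns the explosion particles and destroys the actor.
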(event ComponentTriggered(Comp_Trigger)
  (params (SourceInfo :type Struct%20Component%20Source%20Info%20Structure) (Name :type Name :default "None"))
  (bind _textrender (Variables|Default|GetTextRender))
  (switch name (.identifier SourceInfo)
    (:Button_Start
      (Rendering|Components|TextRender|SetText _textrender (Utilities|Text|ToText(Integer) (Variables|Default|GetTime)))
      (Rendering|SetVisibility _textrender true false)
      (bind _returnvalue (Utilities|Time|SetTimerbyEvent (delegate Custom|Countdown_Main) 1.0 true)))
    (:Button_Stop
      (Utilities|Time|PauseTimerbyHandle _returnvalue))))

(event Custom|Countdown_Main
  (bind _result (Math|Integer|DecrementInt (Variables|Default|GetTime))
    (:%20%20
      (bind _output_get (Variables|Default|SetTime _result))
      (Rendering|Components|TextRender|SetText (Variables|Default|GetTextRender) (Utilities|Text|ToText(Integer) _output_get))
      (if (== (Variables|Default|GetTime) 0)
        (Utilities|Time|ClearandInvalidateTimerbyHandle (stale ComponentTriggered(Comp_Trigger) _returnvalue))
        (CallFunction|Explosion)))))

(event Custom|Explosion
  (bind _sm_bomb (Variables|Default|GetSM_Bomb))
  (bind (_direction _scale _move) (Timeline|Timeline_0 Play)
    (:Update
      (Transformation|SetRelativeScale3D _sm_bomb (Math|Conversions|ToVector(Float) _scale))
      (Utilities|SetRelativeLocationZ _sm_bomb (Math|Float|Lerp 0.0 -2e+02 _move) false false))
    (:Explode
      (Effects|SpawnEmitteratLocation "/Game/AFCore/Examples/Meshes/Bomb/Effect/P_Explosion_Bomb.P_Explosion_Bomb" (Transformation|GetActorLocation))
      (Actor|DestroyActor))))

(event EventBeginPlay)

(event Collision|EventActorBeginOverlap
  (params (OtherActor :type Actor%20Object%20Reference)))

(event EventTick
  (params (DeltaSeconds :type Float%20%28single-precision%29)))

(fn ConstructionScript)