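; BP_ClimbActor_Form is a climbing hold actor with a selectable mesh shape and color, configured entirely in the Construction Script.
; When Randomize is set, it rolls a random mesh index and a color clamped to a mid range.
; The clamped index selects from the Meshes array, and a dynamic instance of the climbing stone master material receives the color.
; The event graph holds no logic.
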(event EventBeginPlay)

(event Collision|EventActorBeginOverlap
  (params (OtherActor :type Actor%20Object%20Reference)))

(event EventTick
  (params (DeltaSeconds :type Float%20%28single-precision%29)))

(fn ConstructionScript
  (bind _returnvalue (Math|Random|RandomUnitVector))
  (bind _meshes (Variables|Default|GetMeshes))
  (bind _returnvalue_2 (Utilities|Array|LastIndex _meshes))
  ;[1 1 1] Set Mesh
  (if (Variables|Default|GetRandomize)
    (Variables|Default|Setcolor (Utilities|Struct|MakeLinearColor (Math|Float|Clamp(Float) (.x _returnvalue) 0.2 0.8) (Math|Float|Clamp(Float) (.y _returnvalue) 0.2 0.8) (Math|Float|Clamp(Float) (.z _returnvalue) 0.2 0.8) 1.0))
    (Variables|Default|SetMeshVariant (Math|Random|RandomIntegerinRange 0 _returnvalue_2)))
  (Variables|Default|SetMeshVariant (Math|Integer|Clamp(Integer) (Variables|Default|GetMeshVariant) 0 _returnvalue_2))
  (Components|StaticMesh|SetStaticMesh (Variables|Default|GetStaticMesh) (Utilities|Array|Get(acopy) (Variables|Default|GetMeshes) (Variables|Default|GetMeshVariant)))
  (bind _returnvalue_3 (Rendering|Material|CreateDynamicMaterialInstance (Variables|Default|GetStaticMesh) 0 "/Game/AVRFramework/Experiences/Demospace/Meshes/Action/Climbing/Mat_ClimbingStone_Master.Mat_ClimbingStone_Master" "None" :!class /Script/Engine.PrimitiveComponent))
  (Rendering|Material|SetVectorParameterValue _returnvalue_3 "color" (Variables|Default|Getcolor) :!class /Script/Engine.MaterialInstanceDynamic))