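; BP_UFO is a selectable vehicle actor that carries a pawn along the spline of a referenced SplineMeshActor.
; Selecting it makes the pawn enter through the vehicle component, which starts a timeline after a short delay.
; The timeline moves the UFO slightly above the spline, with play rate scaled inversely to spline length, and ejects the pawn when finished.
; The construction script snaps it to the spline start.
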(event VehicleEntered(Comp_Vehicle)
  (params (Pawn :type BP%20Pawn%20Base%20Object%20Reference))
  (bind _splinemeshactor (Variables|Default|GetSplineMeshActor))
  (bind _spline (Variables|/Game/AVRFramework/Blueprints/Utility/SplineMesh/BP_SplineMesh.BP_SplineMesh_C|GetSpline _splinemeshactor))
  (Utilities|FlowControl|Delay 1.0)
  (Components|Timeline|SetPlayRate (Variables|Default|GetSplineMovementTimeline) (/ 3e+02 (Spline|GetSplineLength _spline)))
  (bind _percent (Timeline|SplineMovementTimeline PlayFromStart)
    (:Update
      (Transformation|SetActorLocationAndRotation (+ (Spline|GetLocationatTime _spline _percent "World" false) "0, 0,60.000000") (Class|SplineComponent|GetRotationatTime _spline _percent "World" false)))
    (:Finished
      (Default|ExitVehicle (Variables|Default|GetComp_Vehicle)))))

(event VehicleExit(Comp_Vehicle)
  (params (Pawn :type BP%20Pawn%20Base%20Object%20Reference)))

(event PressedSelect(Comp_Select)
  (params (Pawn :type BP%20Pawn%20Base%20Object%20Reference) (MotionControllerActor :type BP%20Motion%20Controller%20Object%20Reference) (MotionController :type Motion%20Controller%20Component%20Object%20Reference) (MComp :type BP%20M%20Comp%20Object%20Reference) (ImpactLocation :type Vector :default "0, 0, 0") (ImpactComponent :type Actor%20Component%20Object%20Reference))
  (Default|EnterVehicle (Variables|Default|GetComp_Vehicle) Pawn))

(event Custom|SetToStartLocation
  (bind _splinemeshactor (Variables|Default|GetSplineMeshActor))
  (bind _spline (Variables|/Game/AVRFramework/Blueprints/Utility/SplineMesh/BP_SplineMesh.BP_SplineMesh_C|GetSpline _splinemeshactor))
  (Transformation|SetActorLocationAndRotation (+ (Spline|GetLocationatTime _spline 0.0 "World" false) "0, 0,60.000000") (Class|SplineComponent|GetRotationatTime _spline 0.0 "World" false)))

(event EventBeginPlay)

(event Collision|EventActorBeginOverlap
  (params (OtherActor :type Actor%20Object%20Reference)))

(event EventTick
  (params (DeltaSeconds :type Float%20%28single-precision%29)))

(fn ConstructionScript
  (Utilities|IsValid (Variables|Default|GetSplineMeshActor)
    (:Is%20Valid
      (CallFunction|SettoStartLocation))))