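; Sci-fi door Blueprint that animates its blades open or closed when its Comp_Active component changes active state.
; Each change plays the matching non-looping animation and mirrors the previous playback position against a fixed length, so interrupted motion reverses from where it was.
; On opening, a Gate is entered before being opened, apparently to skip that position correction the first time.
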(event ActiveStateChanged(Comp_Active)
  (params (Active :type Boolean))
  (bind _scifi_door_blades (Variables|Default|GetSciFi_Door_Blades))
  (Variables|Default|SetCurrentAnimPosition (Class|SkeletalMeshComponent|GetPosition (Variables|Default|GetSciFi_Door_Blades)))
  (if (not Active)
    (Components|Animation|PlayAnimation _scifi_door_blades "/Game/AVRFramework/Experiences/Demospace/Meshes/ArchViz/Architecture/SciFi_Door/SciFi_Door_Blades_Close.SciFi_Door_Blades_Close" false)
    (else
      (Components|Animation|PlayAnimation _scifi_door_blades "/Game/AVRFramework/Experiences/Demospace/Meshes/ArchViz/Architecture/SciFi_Door/SciFi_Door_Open.SciFi_Door_Open" false)
      ;[1 1 1] Set Anim Position if chaged during tha old animation still plays
      (Utilities|FlowControl|Sequence
        (:then_0
          (Utilities|FlowControl|Gate true :!label _label
            (:Exit
              _)))
        (:then_1
          (goto _label Open)))))
  (Components|Animation|SetPosition (Variables|Default|GetSciFi_Door_Blades) (- 2.5 (Variables|Default|GetCurrentAnimPosition)) true))

(event EventBeginPlay)

(event Collision|EventActorBeginOverlap
  (params (OtherActor :type Actor%20Object%20Reference)))

(event EventTick
  (params (DeltaSeconds :type Float%20%28single-precision%29)))

(fn ConstructionScript)