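; BP_BaseballLauncher is an actor that launches baseball projectiles and keeps a count of balls hit.
; A trigger listener component fires SpawnBall, which spawns a projectile at the Arrow's transform and passes the launcher as a reference.
; GiveScore increments Score and updates the Text display, but nothing in this Blueprint calls it.
; An automatic looping-timer spawn mode exists but is disconnected.
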(event TriggerSingle(Comp_ListenToTrigger)
  (params (Name :type Name :default "None") (Section :type Struct%20Section%20Structure) (Source :type Actor%20Object%20Reference) (Pawn :type BP%20Pawn%20Base%20Object%20Reference))
  (CallFunction|SpawnBall))

(event Custom|SpawnBall
  (Game|SpawnActorfromClass "/Game/AVRFramework/Experiences/Demospace/Meshes/Action/Baseball/BP_Baseballball_Projectile.BP_Baseballball_Projectile_C" (Transformation|GetWorldTransform (Variables|Default|GetArrow)) "Undefined" 0 self 0))

(event Custom|GiveScore
  (bind _result (Math|Integer|IncrementInt (Variables|Default|GetScore))
    (:%20%20
      (Rendering|Components|TextRender|SetText (Variables|Default|GetText) (Utilities|Text|ToText(String) (Utilities|String|Append (Utilities|String|ToString(Integer) _result) " Balls hit!"))))))

(event EventBeginPlay)

(fn ConstructionScript)