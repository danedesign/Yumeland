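; BP_ChangeController_Map is a trigger that switches the VR pawn's default controller map preset between teleport and move.
; On overlap with a BP_Pawn_VR, it sets the DefaultPreset on the pawn's CompControllerVR to the teleport or move data asset, chosen by the Teleport flag.
; When UseCollisionbox is off, it destroys its collision component at BeginPlay.
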(event OnComponentBeginOverlap(CollisionComponent)
  (params (OverlappedComponent :type Primitive%20Component%20Object%20Reference) (OtherActor :type Actor%20Object%20Reference) (OtherComp :type Primitive%20Component%20Object%20Reference) (OtherBodyIndex :type Integer) (bFromSweep :type Boolean) (SweepResult :type Hit%20Result%20Structure%20%28by%20ref%29))
  (bind _asbp_pawn_vr (Utilities|Casting|CastToBP_Pawn_VR OtherActor))
  (if (Variables|Default|GetTeleport)
    (Variables|/Game/AVRFramework/Blueprints/Components/Info/Comp_Controls.Comp_Controls_C|SetDefaultPreset (Variables|/Game/AVRFramework/Blueprints/Pawn/BP_Pawn_VR.BP_Pawn_VR_C|GetComp_Controller_VR _asbp_pawn_vr) "/Game/AVRFramework/Experiences/Demospace/DataAssets/Presets/DA_ControllerVR_MapPreset_Teleport.DA_ControllerVR_MapPreset_Teleport")
    (else
      (Variables|/Game/AVRFramework/Blueprints/Components/Info/Comp_Controls.Comp_Controls_C|SetDefaultPreset (Variables|/Game/AVRFramework/Blueprints/Pawn/BP_Pawn_VR.BP_Pawn_VR_C|GetComp_Controller_VR _asbp_pawn_vr) "/Game/AVRFramework/Experiences/Demospace/DataAssets/Presets/DA_ControllerVR_MapPreset_Move.DA_ControllerVR_MapPreset_Move"))))

(event EventBeginPlay
  (if (not (Variables|Default|GetUseCollisionbox))
    (Components|DestroyComponent (Variables|Default|GetCollisionComponent))))

(fn ConstructionScript)