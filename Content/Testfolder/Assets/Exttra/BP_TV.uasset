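; BP_TV is a television Blueprint that plays a video with sound on a plane mesh, driven by an active-state component.
; When Comp_Active turns on it calls InitializePlayer and plays the MediaPlayer, and when it turns off it pauses playback.
; InitializePlayer uses a DoOnce to wire up the media sound and volume, open the video source, set looping and apply the media material to the plane.
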(event ActiveStateChanged(Comp_Active)
  (params (Active :type Boolean))
  (bind _mediaplayer (Variables|Default|GetMediaPlayer))
  ;[1 1 1] Active State Changed
  (if Active
    (|InitializePlayer)
    (Media|MediaPlayer|Play _mediaplayer :!class /Script/MediaAssets.MediaPlayer)
    (else
      (Sequencer|Player|Pause _mediaplayer))))

(event EventBeginPlay
  (|CallParentFunction))

(event Collision|EventActorBeginOverlap
  (params (OtherActor :type Actor%20Object%20Reference))
  (|CallParentFunction OtherActor) ; This node is disabled and will not be called.\nDrag off pins to build functionality.
)

(event EventTick
  (params (DeltaSeconds :type Float%20%28single-precision%29))
  (|CallParentFunction DeltaSeconds) ; This node is disabled and will not be called.\nDrag off pins to build functionality.
)

(fn ConstructionScript
  (|CallParentFunction))