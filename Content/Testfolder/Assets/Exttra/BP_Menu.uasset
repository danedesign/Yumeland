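; Menu actor that spawns a selectable panel for each entry in Levels, on the authority only, as either large or small panels.
; Panel select and unselect events update the selected level, then every panel moves to a recalculated position and only the selected one expands.
; Large panels form a row that re-centers on the clicked level, widening around a selection.
; Small panels form a grid, bringing the selection to a front position.
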(event Custom|PanelSelected
  (params (Panel :type BP%20Panel%20Object%20Reference))
  (bind _panels (Variables|Internal|GetPanels))
  (bind (_value _returnvalue) (Utilities|Map|Find _panels Panel))
  ;[1 1 1] Create and Setup all Panels according to Experiences specified in the Universal object
  (if _returnvalue
    (CallFunction|LevelSelected _value)))

(event Custom|LevelSelected
  (params (Level :type BP%20Info%20Level%20Class%20Reference))
  (bind _levels (Variables|Settings|GetLevels))
  ;[1 1 1] New Level Selected
  (Utilities|FlowControl|Sequence
    (:then_0
      (switch Utilities|FlowControl|Switch|SwitchonEnum_Menu_Type (Variables|Settings|GetMenuType)
        (:NewEnumerator0
          (if (Utilities|IsValidClass Level)
            (if (<= (Math|Integer|Absolute(Integer) (- (Utilities|Array|FindItem _levels Level) (Utilities|Array|FindItem _levels (Variables|Settings|GetCenteredLevel)))) 1)
              (Variables|Internal|SetSelectedLevel Level)
              (else
                (Variables|Internal|SetSelectedLevel 0)))
            (Variables|Settings|SetCenteredLevel Level)
            (else
              (Variables|Internal|SetSelectedLevel 0))))
        (:NewEnumerator1
          (Variables|Internal|SetSelectedLevel Level))))
    (:then_1
      (CallFunction|ArrangePanels))))

(event Custom|PanelUnselected
  (params (Panel :type BP%20Panel%20Object%20Reference))
  ;[1 1 1] Create and Setup all Panels according to Experiences specified in the Universal object
  (if (.ReturnValue (Utilities|Map|Find (Variables|Internal|GetPanels) Panel))
    (CallFunction|LevelSelected)))

(event Custom|ArrangePanels
  (bind _panels (Variables|Internal|GetPanels))
  ;[1 1 1] Arrange all Panels
  (bind _keys (Utilities|Map|Keys _panels))
  (for _array_element _keys
    (if (.ReturnValue (Utilities|Map|Find _panels _array_element))
      (Default|MultiMovetoLocation _array_element 1.0 (CallFunction|CalculatePosition (.Value (Utilities|Map|Find _panels _array_element))))
      (if (== (.Value (Utilities|Map|Find _panels _array_element)) (Variables|Internal|GetSelectedLevel))
        (Default|MultiExpand _array_element true)
        (else
          (Default|MultiExpand _array_element false))))))

(event EventBeginPlay
  (bind _menutype (Variables|Settings|GetMenuType))
  ;[1 1 1] Create and Setup all Panels according to Experiences specified in the Universal object
  (Networking|SwitchHasAuthority
    (:Authority
      (for _array_element (Variables|Settings|GetLevels)
        (bind _asbp_panel (Utilities|Casting|CastToBP_PanelClass (Utilities|Select :Index _menutype :NewEnumerator0 "/Game/AVRFramework/Blueprints/UI/Panel/BP_Panel_Large.BP_Panel_Large_C" :NewEnumerator1 "/Game/AVRFramework/Blueprints/UI/Panel/BP_Panel_Small.BP_Panel_Small_C")))
        (bind _returnvalue (Game|SpawnActorfromClass _asbp_panel (CallFunction|CalculatePosition _array_element) "Undefined" self false _menutype _array_element 0))
        (Utilities|Map|Add (Variables|Internal|GetPanels) _returnvalue _array_element)
        (Transformation|AttachActorToActor _returnvalue self "None" "KeepWorld" "KeepWorld" "KeepWorld" true)
        (EventDispatchers|AssignPanelSelected _returnvalue (delegate Custom|PanelSelected))
        (EventDispatchers|AssignPanelUnselected _returnvalue (delegate Custom|PanelUnselected)))
      (CallFunction|ArrangePanels))))

(fn ConstructionScript)

(fn CalculatePosition
  (params (Level :type BP%20Info%20Level%20Class%20Reference%20%28by%20ref%29))
  (bind _returnvalue (Math|Float|MakeLiteralFloat 325.0))
  (bind _itemperrow (Variables|Settings|GetItemPerRow))
  (bind _levels (Variables|Settings|GetLevels))
  (bind _levels_2 (Variables|Settings|GetLevels))
  (bind _centeredlevel (Variables|Settings|GetCenteredLevel))
  (bind _levels_3 (Variables|Settings|GetLevels))
  (bind _frontposition (Variables|Default|GetFrontPosition))
  (bind _returnvalue_2 (Utilities|Array|FindItem _levels_3 Level))
  (bind _returnvalue_3 (Utilities|Array|FindItem _levels Level))
  (bind _returnvalue_4 (Utilities|Array|FindItem _levels_2 _centeredlevel))
  (bind _returnvalue_5 (Class|KismetSystemLibrary|MakeLiteralInteger _itemperrow))
  (bind _returnvalue_6 (Transformation|GetWorldTransform _frontposition))
  (bind (_location _rotation _scale) (Math|Transform|BreakTransform _returnvalue_6))
  (bind _returnvalue_7 (- _returnvalue_4 _returnvalue_2))
  (bind _returnvalue_8 (Math|Conversions|ToFloat(Integer) _returnvalue_7))
  (switch Utilities|FlowControl|Switch|SwitchonEnum_Menu_Type (Variables|Settings|GetMenuType)
    (:NewEnumerator0
      (Transformation|SetRelativeTransform (Variables|Default|GetPositionHelper) (Math|Transform|MakeTransform (Math|Vector|MakeVector 0.0 (* (select (Utilities|IsValidClass (Variables|Internal|GetSelectedLevel)) (select (== _returnvalue_7 0) 0.0 (+ _returnvalue_8 (select (< _returnvalue_8 0.0) -0.75 0.75))) _returnvalue_8) 768.0) 0.0) "0, 0, 0" "1,1,1") false false)
      (return (Transformation|GetWorldTransform (Variables|Default|GetPositionHelper))))
    (:NewEnumerator1
      (if (== (Variables|Internal|GetSelectedLevel) Level)
        (return (Math|Transform|MakeTransform _location _rotation _scale))
        (else
          (Transformation|SetRelativeTransform (Variables|Default|GetPositionHelper) (Math|Transform|MakeTransform (Math|Vector|MakeVector 0.0 (- (- (/ (* _returnvalue_5 _returnvalue) 2.0) (/ _returnvalue 2.0)) (* (Math|Integer|%(Integer) _returnvalue_3 _returnvalue_5) _returnvalue)) (* (/ _returnvalue_3 _returnvalue_5) _returnvalue)) "0, 0, 0" (Math|Conversions|ToVector(Float) (Math|Float|MakeLiteralFloat 0.5))) false false)
          (return (Transformation|GetWorldTransform (Variables|Default|GetPositionHelper))))))))