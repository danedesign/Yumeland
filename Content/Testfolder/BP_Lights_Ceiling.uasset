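; BP_Lights_Ceiling is a ceiling light actor whose spot light fades on and off with an active state.
; Comp_Active's state change plays or reverses LightTimeline, whose Percent output interpolates the SpotLight intensity between dark and full brightness.
; An in-editor state change calls ManipulateTimeline toward the matching end, then applies the intensity directly through the same logic.
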(event ActiveStateChanged(Comp_Active)
  (params (SourceInfo :type Struct%20Component%20Source%20Info%20Structure) (Active :type Boolean))
  (if Active
    (bind _percent (Timeline|LightTimeline Play)
      (:Update
        (Rendering|Components|Light|SetIntensity (Variables|Default|GetSpotLight) (Math|Float|Lerp 0.0 1e+04 _percent))))
    (else
      (Timeline|LightTimeline Reverse))))

(event InEditorActiveStateChanged(Comp_Active)
  (params (Active :type Boolean))
  (Utilities|ManipulateTimeline (Variables|Default|GetLightTimeline) Active)
  (Rendering|Components|Light|SetIntensity (Variables|Default|GetSpotLight) (Math|Float|Lerp 0.0 1e+04 (stale ActiveStateChanged(Comp_Active) _percent))))

(event EventBeginPlay
  (|CallParentFunction) ; This node is disabled and will not be called.\nDrag off pins to build functionality.
)

(event Collision|EventActorBeginOverlap
  (params (OtherActor :type Actor%20Object%20Reference))
  (|CallParentFunction OtherActor) ; This node is disabled and will not be called.\nDrag off pins to build functionality.
)

(event EventTick
  (params (DeltaSeconds :type Float%20%28single-precision%29))
  (|CallParentFunction DeltaSeconds))

(fn ConstructionScript
  (|CallParentFunction))