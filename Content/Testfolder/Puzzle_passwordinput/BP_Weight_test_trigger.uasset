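; Test puzzle actor with a barbell plate mesh that changes color, tilts and grows while its CompActive Active value is true.
; Tick requests a dynamic material instance, then a Delay throttles the effect to roughly every 0.2 seconds.
; Each pass randomizes ColorMain, prints a debug string and increments the plate's pitch and scale with no upper limit.
; BeginPlay clears Inputcorrect, which is never read here.
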(event EventBeginPlay
  (Variables|Default|SetInputcorrect? false))

(event Collision|EventActorBeginOverlap
  (params (OtherActor :type Actor%20Object%20Reference)))

(event EventTick
  (params (DeltaSeconds :type Float%20%28single-precision%29))
  (bind _sm_barbell_plate_standart_10_lp (Variables|Default|GetSM_Barbell_Plate_Standart_10_LP))
  (bind _sm_barbell_plate_standart_10_lp_2 (Variables|Default|GetSM_Barbell_Plate_Standart_10_LP))
  (bind _returnvalue (Transformation|GetWorldRotation _sm_barbell_plate_standart_10_lp_2))
  (if (.value (Variables|/Game/AFCore/Blueprints/Components/State/Comp_Active.Comp_Active_C|GetActive (Variables|Default|GetComp_Active)))
    (bind _returnvalue_2 (Rendering|Material|CreateDynamicMaterialInstance _sm_barbell_plate_standart_10_lp 0 (Rendering|Material|GetMaterial _sm_barbell_plate_standart_10_lp 0) "None" :!class /Script/Engine.PrimitiveComponent))
    (Utilities|FlowControl|Delay (+ DeltaSeconds 0.2))
    (Rendering|Material|SetVectorParameterValue _returnvalue_2 "ColorMain" (Utilities|Struct|MakeLinearColor (Math|Random|RandomFloatinRange 0.0 1.0) (Math|Random|RandomFloatinRange 0.0 1.0) (Math|Random|RandomFloatinRange 0.0 1.0) (Math|Random|RandomFloatinRange 0.0 1.0)) :!class /Script/Engine.MaterialInstanceDynamic)
    (Development|PrintString "??????")
    (Transformation|SetWorldTransform _sm_barbell_plate_standart_10_lp_2 (Math|Transform|MakeTransform (Transformation|GetWorldLocation _sm_barbell_plate_standart_10_lp_2) (Math|Rotator|MakeRotator (.roll _returnvalue) (+ (.pitch _returnvalue) 1.0) (.yaw _returnvalue)) (+ (Transformation|GetWorldScale _sm_barbell_plate_standart_10_lp_2) "0.200000,0.200000,0.200000")) false false)))

(fn ConstructionScript)