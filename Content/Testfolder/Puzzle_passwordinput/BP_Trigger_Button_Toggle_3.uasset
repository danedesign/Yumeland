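; Toggle button for a password-input puzzle that acts as input C, the third in the order.
; Active-state changes on Comp_Active set or clear PasswordC and Order03, and play or reverse ColorTimeline.
; The timeline blends the button's color from red to green and raises its Fresnel exponent through a lazily created dynamic material instance.
; An in-editor state handler snaps the timeline to preview the matching look.
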(event InEditorActiveStateChanged(Comp_Active)
  (params (Active :type Boolean))
  (Utilities|ManipulateTimeline (Variables|Default|GetColorTimeline) Active)
  ;[1 1 1] ButtonColorChange
  (CallFunction|SetButtonColor (stale ActiveStateChanged(Comp_Active) _procent)))

(event ActiveStateChanged(Comp_Active)
  (params (SourceInfo :type Struct%20Component%20Source%20Info%20Structure) (Active :type Boolean))
  ;[1 1 1] ButtonColorChange
  (if Active
    (Variables|Default|Setpassword_C true)
    (Variables|Default|Setorder_03 3)
    (bind _procent (Timeline|ColorTimeline Play)
      (:Update
        (CallFunction|SetButtonColor _procent)))
    (else
      (Variables|Default|Setpassword_C false)
      (Variables|Default|Setorder_03 0)
      (Timeline|ColorTimeline Reverse))))

(event EventBeginPlay
  (Variables|Default|Setpassword_C false))

(fn ConstructionScript)

(fn SetButtonColor
  (params (Alpha :type Float%20%28single-precision%29))
  (bind _material (CallFunction|GetButtonMaterial))
  (Rendering|Material|SetVectorParameterValue _material "Color" (Math|Color|Lerp(LinearColor) "(R=1.000000,G=0.000000,B=0.000000,A=1.000000)" "(R=0.000000,G=1.000000,B=0.000000,A=1.000000)" Alpha) :!class /Script/Engine.MaterialInstanceDynamic)
  (Rendering|Material|SetScalarParameterValue _material "FresnelExponent" (Math|Float|Lerp 0.3 2.0 Alpha) :!class /Script/Engine.MaterialInstanceDynamic))

(fn GetButtonMaterial
  (Variables|Default|GetButtonMaterial
    (:then
      _)
    (:else
      (bind _returnvalue (Rendering|Material|CreateDynamicMaterialInstance (Variables|Default|GetMesh_Button_Button) 0 "/Game/AFCore/Examples/Meshes/UnrealButton/MI_Button_Logo_Door.MI_Button_Logo_Door" "None" :!class /Script/Engine.PrimitiveComponent))
      (Variables|Default|SetButtonMaterial _returnvalue)))
  (return (Variables|Default|GetButtonMaterial)))