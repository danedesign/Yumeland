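; BP_Ore_Refinery_Platform is an ore refinery platform that tracks when it becomes active for war mining.
; Attachment events on two anchor pipe components set a tunnel flag for each pipe.
; A looping half-second timer started at BeginPlay polls both flags and sets WarMiningHere once both tunnels are attached; nothing here clears it.
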(event ActorGotAttached(Comp_Anchor_Pipe_1)
  (params (Anchor :type Comp%20Anchor%20Object%20Reference) (Actor :type Actor%20Object%20Reference) (Connector :type Comp%20Connector%20Anchor%20Object%20Reference))
  (Variables|Default|SetTunnel_01 true))

(event ActorGotAttached(Comp_Anchor_Pipe_2)
  (params (Anchor :type Comp%20Anchor%20Object%20Reference) (Actor :type Actor%20Object%20Reference) (Connector :type Comp%20Connector%20Anchor%20Object%20Reference))
  (Variables|Default|SetTunnel_02 true))

(event Custom|ActiveWarMining
  (if (and (Variables|Default|GetTunnel_01) (Variables|Default|GetTunnel_02))
    (Variables|Default|SetWarMiningHere! true)))

(event EventBeginPlay
  (Utilities|Time|SetTimerbyEvent (delegate Custom|ActiveWarMining) 0.5 true))

(fn ConstructionScript)