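; BP_Radio is a puzzle radio that streams looping music through a media sound component.
; Attaching actors to its three anchor components sets one flag each.
; A looping half-second timer polls those flags and sets Active once all three are true.
; The active component's state plays or pauses the media player, both on BeginPlay and whenever that state changes.
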(event ActiveStateChanged(Comp_Active)
  (params (SourceInfo :type Struct%20Component%20Source%20Info%20Structure) (Active :type Boolean))
  (bind _mediasound (Variables|Default|GetMediaSound))
  (bind _returnvalue (Class|MediaSoundComponent|GetMediaPlayer _mediasound))
  (if Active
    (Media|MediaPlayer|Play _returnvalue :!class /Script/MediaAssets.MediaPlayer)
    (else
      (Sequencer|Player|Pause _returnvalue))))

(event ActorGotAttached(Comp_Anchor)
  (params (Anchor :type Comp%20Anchor%20Object%20Reference) (Actor :type Actor%20Object%20Reference) (Connector :type Comp%20Connector%20Anchor%20Object%20Reference))
  (Variables|Default|SetButton_01? true))

(event ActorGotAttached(Comp_Anchor1)
  (params (Anchor :type Comp%20Anchor%20Object%20Reference) (Actor :type Actor%20Object%20Reference) (Connector :type Comp%20Connector%20Anchor%20Object%20Reference))
  (Variables|Default|SetButton_02? true))

(event ActorGotAttached(Comp_Anchor2)
  (params (Anchor :type Comp%20Anchor%20Object%20Reference) (Actor :type Actor%20Object%20Reference) (Connector :type Comp%20Connector%20Anchor%20Object%20Reference))
  (Variables|Default|SetButton_03? true))

(event Custom|Active
  (if (Math|Boolean|ANDBoolean (Variables|Default|GetButton_01?) (Variables|Default|GetButton_02?) (Variables|Default|GetButton_03?))
    (Variables|Default|Setactive! true)))

(event EventBeginPlay
  (bind _mediasound (Variables|Default|GetMediaSound))
  (bind _returnvalue (Class|MediaSoundComponent|GetMediaPlayer _mediasound))
  (Utilities|Time|SetTimerbyEvent (delegate Custom|Active) 0.5 true)
  (Media|MediaPlayer|OpenSourcewithOptions _returnvalue "/Game/AFCore/Examples/Meshes/Radio/Radio_Music_StreamExample.Radio_Music_StreamExample" (Utilities|Struct|MakeMediaPlayerOptions "(Audio=0,Caption=-1,Metadata=-1,Script=-1,Subtitle=-1,Text=-1,Video=0)" "+00000000.00:00:00.000000000" "Disabled" "Enabled") :!class /Script/MediaAssets.MediaPlayer)
  (if (.value (Variables|/Game/AFCore/Blueprints/Components/State/Comp_Active.Comp_Active_C|GetActive (Variables|Default|GetComp_Active)))
    (Media|MediaPlayer|Play _returnvalue :!class /Script/MediaAssets.MediaPlayer)
    (else
      (Sequencer|Player|Pause _returnvalue))))

(fn ConstructionScript)