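; Gaze-reactive narrative object that turns its text label and background toward the desktop player when viewed.
; On the gaze component's GazeView event, it casts the pawn to BP_Pawn_Desktop and reads the CameraHandle's world yaw.
; TextRender and Background both take that yaw plus 180 degrees with zero roll, billboarding only when the event fires, as Tick is unused.
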(event GazeView(Comp_Gaze)
  (params (Set :type Boolean) (Pawn :type BP%20Pawn%20Base%20Object%20Reference) (ImpactLocation :type Vector :default "0, 0, 0") (ImpactRotation :type Rotator :default "0, 0, 0"))
  (bind _new_rotation_y__pitch_ (Variables|Default|GetNew%20Rotation%20Y%20%28Pitch%29))
  (bind _asbp_pawn_desktop (Utilities|Casting|CastToBP_Pawn_Desktop Pawn))
  (Transformation|SetWorldRotation (Variables|Default|GetTextRender) (Math|Rotator|MakeRotator 0.0 _new_rotation_y__pitch_ (+ (* (.yaw (Transformation|GetWorldRotation (Variables|/Game/AFCore/Blueprints/Pawn/BP_Pawn_Base.BP_Pawn_Base_C|GetCameraHandle _asbp_pawn_desktop))) 1.0) 1.8e+02)) false false)
  (Transformation|SetWorldRotation (Variables|Default|GetBackground) (Math|Rotator|MakeRotator 0.0 _new_rotation_y__pitch_ (+ (* (.yaw (Transformation|GetWorldRotation (Variables|/Game/AFCore/Blueprints/Pawn/BP_Pawn_Base.BP_Pawn_Base_C|GetCameraHandle _asbp_pawn_desktop))) 1.0) 1.8e+02)) false false))

(event EventBeginPlay)

(event Collision|EventActorBeginOverlap
  (params (OtherActor :type Actor%20Object%20Reference)))

(event EventTick
  (params (DeltaSeconds :type Float%20%28single-precision%29)))

(fn ConstructionScript
  (|CallParentFunction))