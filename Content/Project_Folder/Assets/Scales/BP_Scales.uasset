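; BP_Scales is a balance scale actor that tips once when an actor is attached to its anchor component.
; On BeginPlay it hides the Indicator and spawns an attached BP_Helper_MeshCopy that copies its meshes with an outline highlight material.
; The first attachment sets WeightAttached, briefly shows and scales the Indicator before destroying it, and plays timelines that incrementally roll the stand and shift both balance pieces.
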(event ActorGotAttached(Comp_Anchor)
  (params (Anchor :type Comp%20Anchor%20Object%20Reference) (Actor :type Actor%20Object%20Reference) (Connector :type Comp%20Connector%20Anchor%20Object%20Reference))
  (bind _indicator (Variables|Default|GetIndicator))
  (bind _returnvalue (Transformation|GetWorldTransform _indicator))
  (Utilities|FlowControl|DoOnce false
    (:Completed
      (Variables|Default|SetWeightAttached? true)
      (Utilities|FlowControl|Sequence
        (:then_0
          (Variables|Default|SetWeightAttached? true)
          (Rendering|SetVisibility _indicator true false)
          (bind _newtrack_0 (Timeline|Timeline_3 Play)
            (:Update
              (Transformation|SetWorldTransform _indicator (Math|Transform|MakeTransform (.location _returnvalue) (.rotation _returnvalue) (Math|Vector|MakeVector _newtrack_0 (.y (.scale _returnvalue)) _newtrack_0)) false false)
              (Utilities|FlowControl|Delay 1.0)
              (Components|DestroyComponent _indicator))))
        (:then_1
          (bind _newtrack_0_2 (Timeline|Timeline_2 Play)
            (:Update
              (Class|SceneComponent|AddWorldTransform (Variables|Default|Getscales_stand) (Math|Transform|MakeTransform "0, 0, 0" (Math|Rotator|MakeRotator _newtrack_0_2 0.0 0.0) "1,1,1") false false))))
        (:then_2
          (bind (_direction _z _y) (Timeline|Timeline_0 Play)
            (:Update
              (Class|SceneComponent|AddWorldTransform (Variables|Default|Getscales_scales_balance_1) (Math|Transform|MakeTransform (Math|Vector|MakeVector 0.0 _y _z) "0, 0, 0" "1,1,1") false false))))
        (:then_3
          (bind (_direction_2 _y_2 _z_2) (Timeline|Timeline_1 Play)
            (:Update
              (Class|SceneComponent|AddWorldTransform (Variables|Default|Getscales_scales_balance_2) (Math|Transform|MakeTransform (Math|Vector|MakeVector 0.0 _y_2 _z_2) "0, 0, 0" "1,1,1") false false))))))))

(event EventBeginPlay
  (bind _self self)
  (bind _defaultsceneroot (Variables|Default|GetDefaultSceneRoot))
  (bind _returnvalue (Transformation|GetWorldTransform _defaultsceneroot))
  (Rendering|SetVisibility (Variables|Default|GetIndicator) false false)
  (bind _returnvalue_2 (Game|SpawnActorfromClass "/Game/AFCore/Blueprints/Helpers/BP_Helper_MeshCopy.BP_Helper_MeshCopy_C" (Math|Transform|MakeTransform (.location _returnvalue) (.rotation _returnvalue) (.scale _returnvalue)) "AlwaysSpawn" 0 (Utilities|Array|MakeArray (Variables|Default|Getscales_scales_balance_1) (Variables|Default|Getscales_scales_balance_2) (Variables|Default|Getmesh) (Variables|Default|Getscales_platform)) "/Game/Testfolder/Virtualization_test/MI_Highlight_Outline_Mesh_Simple_outliner_thinner.MI_Highlight_Outline_Mesh_Simple_outliner_thinner" "(R=0.000000,G=0.000000,B=0.000000,A=1.000000)" false 1.0 _self 0))
  (Transformation|AttachActorToActor _returnvalue_2 _self "None" "KeepWorld" "KeepWorld" "KeepWorld" true))

(event Collision|EventActorBeginOverlap
  (params (OtherActor :type Actor%20Object%20Reference)))

(event EventTick
  (params (DeltaSeconds :type Float%20%28single-precision%29)))

(fn ConstructionScript)