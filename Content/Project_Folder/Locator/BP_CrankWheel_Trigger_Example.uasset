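; BP_CrankWheel_Trigger_Example is an example interactive crank that turns the VR pawn's view when dragged.
; On BeginPlay it spawns and attaches a BP_Helper_MeshCopy that duplicates the crank and wheel meshes with a highlight outline material.
; Comp_Drag's DragStateChangedConstant event adds its Distance value to the yaw of the player BP_Pawn_VR's CameraHandle, keeping pitch and roll.
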(event DragStateChangedConstant(Comp_Drag)
  (params (Name :type Name :default "None") (Distance :type Float%20%28single-precision%29) (Procent :type Float%20%28single-precision%29) (Velocity :type Float%20%28single-precision%29) (Source :type Actor%20Object%20Reference) (Pawn :type BP%20Pawn%20Base%20Object%20Reference))
  (bind _asbp_pawn_vr (Utilities|Casting|CastToBP_Pawn_VR (Game|GetPlayerCharacter 0)))
  (Transformation|SetWorldRotation (Variables|/Game/AFCore/Blueprints/Pawn/BP_Pawn_Base.BP_Pawn_Base_C|GetCameraHandle _asbp_pawn_vr) (Math|Rotator|MakeRotator (.roll (Transformation|GetWorldRotation (Variables|/Game/AFCore/Blueprints/Pawn/BP_Pawn_Base.BP_Pawn_Base_C|GetCameraHandle _asbp_pawn_vr))) (.pitch (Transformation|GetWorldRotation (Variables|/Game/AFCore/Blueprints/Pawn/BP_Pawn_Base.BP_Pawn_Base_C|GetCameraHandle _asbp_pawn_vr))) (+ Distance (.yaw (Transformation|GetWorldRotation (Variables|/Game/AFCore/Blueprints/Pawn/BP_Pawn_Base.BP_Pawn_Base_C|GetCameraHandle _asbp_pawn_vr))))) false false))

(event EventBeginPlay
  (bind _self self)
  (bind _sm_interactive_crank (Variables|Default|GetSM_Interactive_Crank))
  (bind _returnvalue (Transformation|GetWorldTransform _sm_interactive_crank))
  (bind _returnvalue_2 (Game|SpawnActorfromClass "/Game/AFCore/Blueprints/Helpers/BP_Helper_MeshCopy.BP_Helper_MeshCopy_C" (Math|Transform|MakeTransform (.location _returnvalue) (.rotation _returnvalue) (.scale _returnvalue)) "AlwaysSpawn" 0 (Utilities|Array|MakeArray _sm_interactive_crank (Variables|Default|GetSM_Interactive_Crank_Wheel)) "/Game/Testfolder/Virtualization_test/MI_Highlight_Outline_Mesh_Simple_outliner_thinner.MI_Highlight_Outline_Mesh_Simple_outliner_thinner" "(R=0.000000,G=0.000000,B=0.000000,A=1.000000)" false 1.0 _self 0))
  (Transformation|AttachActorToActor _returnvalue_2 _self "None" "KeepWorld" "KeepWorld" "KeepWorld" true))

(event Collision|EventActorBeginOverlap
  (params (OtherActor :type Actor%20Object%20Reference)))

(event EventTick
  (params (DeltaSeconds :type Float%20%28single-precision%29)))

(fn ConstructionScript)