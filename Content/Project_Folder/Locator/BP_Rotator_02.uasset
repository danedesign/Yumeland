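; Locator button actor that nudges the player's camera handle on BP_Pawn_Base by a fixed negative yaw step when activated.
; Active-state events from its active component drive the rotation and a debug print, while deactivation reverses the color timeline.
; Color updates lerp tint and Fresnel exponent on a lazily created dynamic material, then switch the component off after a short delay.
; The in-editor state event also drives the timeline and color update.
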(event InEditorActiveStateChanged(Comp_Active)
  (params (Active :type Boolean))
  (Utilities|ManipulateTimeline (Variables|Default|GetColorTimeline) Active)
  (CallFunction|SetButtonColor (stale ActiveStateChanged(Comp_Active) _procent))
  (Utilities|FlowControl|Delay 0.2)
  (Default|SetActiv (Variables|Default|GetComp_Active)))

(event ActiveStateChanged(Comp_Active)
  (params (SourceInfo :type Struct%20Component%20Source%20Info%20Structure) (Active :type Boolean))
  ;[1 1 1] ButtonColorChange
  (bind _output_get (Variables|Default|Setpresscheck Active))
  (if _output_get
    (Development|PrintString "Hello")
    (bind _asbp_pawn_base (Utilities|Casting|CastToBP_Pawn_Base (Game|GetPlayerCharacter 0)))
    (Transformation|SetWorldRotation (Variables|/Game/AFCore/Blueprints/Pawn/BP_Pawn_Base.BP_Pawn_Base_C|GetCameraHandle _asbp_pawn_base) (Math|Rotator|MakeRotator (.roll (Transformation|GetWorldRotation (Variables|/Game/AFCore/Blueprints/Pawn/BP_Pawn_Base.BP_Pawn_Base_C|GetCameraHandle _asbp_pawn_base))) (.pitch (Transformation|GetWorldRotation (Variables|/Game/AFCore/Blueprints/Pawn/BP_Pawn_Base.BP_Pawn_Base_C|GetCameraHandle _asbp_pawn_base))) (+ (.yaw (Transformation|GetWorldRotation (Variables|/Game/AFCore/Blueprints/Pawn/BP_Pawn_Base.BP_Pawn_Base_C|GetCameraHandle _asbp_pawn_base))) -1e+01)) false false)
    (else
      (bind _procent (Timeline|ColorTimeline Reverse)
        (:Update
          (CallFunction|SetButtonColor _procent)
          (Utilities|FlowControl|Delay 0.2)
          (Default|SetActiv (Variables|Default|GetComp_Active)))))))

(event EventBeginPlay
  (Variables|Default|Setpassword_A false))

(fn ConstructionScript)

(fn SetButtonColor
  (params (Alpha :type Float%20%28single-precision%29))
  (bind _material (CallFunction|GetButtonMaterial))
  (Rendering|Material|SetVectorParameterValue _material "Color" (Math|Color|Lerp(LinearColor) "(R=0.346704,G=1.000000,B=0.737911,A=1.000000)" "(R=0.109462,G=0.238398,B=1.000000,A=1.000000)" Alpha) :!class /Script/Engine.MaterialInstanceDynamic)
  (Rendering|Material|SetScalarParameterValue _material "FresnelExponent" (Math|Float|Lerp 0.3 2.0 Alpha) :!class /Script/Engine.MaterialInstanceDynamic))

(fn GetButtonMaterial
  (Variables|Default|GetButtonMaterial
    (:then
      _)
    (:else
      (bind _returnvalue (Rendering|Material|CreateDynamicMaterialInstance (Variables|Default|GetMesh_Button_Button) 0 "/Game/Project_Folder/Room_01_level_01/Puzzle_passwordinput/Button_toggle_01/M_Button_Logo_01.M_Button_Logo_01" "None" :!class /Script/Engine.PrimitiveComponent))
      (Variables|Default|SetButtonMaterial _returnvalue)))
  (return (Variables|Default|GetButtonMaterial)))