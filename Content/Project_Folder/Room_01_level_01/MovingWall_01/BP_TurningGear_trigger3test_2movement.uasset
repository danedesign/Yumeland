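; Test actor for the Room 01 moving wall that shifts its static mesh along local Z, by velocity input or automatically.
; Comp_Velocity change events add a local transform to the mesh, with Z scaled from the reported velocity.
; A fixed delay after BeginPlay, Automoving plays a timeline that adds Z offsets each update, and the actor destroys itself a few seconds later.
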(event VelocityChanged(Comp_Velocity)
  (params (SourceInfo :type Struct%20Component%20Source%20Info%20Structure) (Value :type Struct%20Velocity%20Structure))
  (Class|SceneComponent|AddLocalTransform (Variables|Default|GetStaticMesh) (Math|Transform|MakeTransform (Math|Vector|MakeVector 0.0 0.0 (* (.velocity Value) 0.2)) "0, 0, 0" (Transformation|GetWorldScale (Variables|Default|GetStaticMesh))) false false))

(event Custom|Automoving
  ;[1 1 1] Autodestroy
  (bind _newtrack_0 (Timeline|Timeline_0 Play)
    (:Update
      (Transformation|AddLocalOffset (Variables|Default|GetStaticMesh) (Math|Vector|MakeVector 0.0 0.0 _newtrack_0) false false))))

(event EventBeginPlay
  ;[1 1 1] Autodestroy
  (Utilities|FlowControl|Delay 5e+01)
  (CallFunction|Automoving)
  (Utilities|FlowControl|Delay 3.2)
  (Actor|DestroyActor))

(event Collision|EventActorBeginOverlap
  (params (OtherActor :type Actor%20Object%20Reference)))

(event EventTick
  (params (DeltaSeconds :type Float%20%28single-precision%29)))

(fn ConstructionScript)