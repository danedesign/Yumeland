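; Moving wall actor for a level room that slides along world X once its active component is triggered.
; The component's state-change event sets its active state, and its activation plays a timeline.
; The timeline curve drives absolute X location while keeping the root's current Y and Z.
; Disconnected leftovers include a second Z-axis door timeline and a speed-based gate-raising routine, neither of which runs.
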(event ActiveStateChanged(Comp_Active)
  (params (SourceInfo :type Struct%20Component%20Source%20Info%20Structure) (Active :type Boolean))
  ;[1 1 1] Set activ
  (Components|Activation|SetActive (Variables|Default|GetComp_Active) Active false))

(event OnComponentActivated(Comp_Active)
  (params (Component :type Actor%20Component%20Object%20Reference) (bReset :type Boolean))
  (bind _defaultsceneroot (Variables|Default|GetDefaultSceneRoot))
  (bind _returnvalue (Transformation|GetWorldLocation _defaultsceneroot))
  ;[1 1 1] Activ then do actions
  ;[1 1 1] Activ then do actions
  (bind _newtrack_0 (Timeline|Timeline_0 Play)
    (:Update
      (bind _output_get (Variables|Default|SetNew%20Location%20Z_actor _newtrack_0))
      (Transformation|SetActorLocation (Math|Vector|MakeVector _output_get (.y _returnvalue) (.z _returnvalue)) false false))))

(event EventBeginPlay)

(event Collision|EventActorBeginOverlap
  (params (OtherActor :type Actor%20Object%20Reference)))

(fn ConstructionScript)