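; A crank wheel interactive for Room 01, level 01, that triggers a voice-line sequence once it is dragged almost fully.
; On BeginPlay it spawns and attaches a BP_Helper_MeshCopy that copies the crank and wheel meshes with an outline highlight material.
; The drag component's progress event fires a DoOnce past 90%, then plays three timed 2D voice prompts separated by delays.
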(event DragStateChangedConstant(Comp_Drag)
  (params (Name :type Name :default "None") (Distance :type Float%20%28single-precision%29) (Procent :type Float%20%28single-precision%29) (Velocity :type Float%20%28single-precision%29) (Source :type Actor%20Object%20Reference) (Pawn :type BP%20Pawn%20Base%20Object%20Reference))
  (if (> Procent 0.9)
    (Utilities|FlowControl|DoOnce false
      (:Completed
        (Utilities|FlowControl|Delay 2.0)
        (Audio|SpawnSound2D "/Game/Project_Folder/Assets/01_Sounds/VoiceOver/Task05/Fixed/Lets_not_lose_our_focus_shall_we.Lets_not_lose_our_focus_shall_we" 1.0 1.0 0.0 0)
        (Utilities|FlowControl|Delay 11.0)
        (Audio|SpawnSound2D "/Game/Project_Folder/Assets/01_Sounds/VoiceOver/Task06/1_Involve_player_to_touch.1_Involve_player_to_touch" 1.0 1.0 0.0 0)
        (Utilities|FlowControl|Delay 1e+01)
        (Audio|SpawnSound2D "/Game/Project_Folder/Assets/01_Sounds/VoiceOver/Task06/2_Touch_the_correct_square.2_Touch_the_correct_square" 1.0 1.0 0.0 0)))))

(event EventBeginPlay
  (bind _self self)
  (bind _sm_interactive_crank (Variables|Default|GetSM_Interactive_Crank))
  (bind _returnvalue (Transformation|GetWorldTransform _sm_interactive_crank))
  (bind _returnvalue_2 (Game|SpawnActorfromClass "/Game/AFCore/Blueprints/Helpers/BP_Helper_MeshCopy.BP_Helper_MeshCopy_C" (Math|Transform|MakeTransform (.location _returnvalue) (.rotation _returnvalue) (.scale _returnvalue)) "AlwaysSpawn" 0 (Utilities|Array|MakeArray _sm_interactive_crank (Variables|Default|GetSM_Interactive_Crank_Wheel)) "/Game/Testfolder/Virtualization_test/MI_Highlight_Outline_Mesh_Simple_outliner_thinner.MI_Highlight_Outline_Mesh_Simple_outliner_thinner" "(R=0.000000,G=0.000000,B=0.000000,A=1.000000)" false 1.0 _self 0))
  (Transformation|AttachActorToActor _returnvalue_2 _self "None" "KeepWorld" "KeepWorld" "KeepWorld" true))

(event Collision|EventActorBeginOverlap
  (params (OtherActor :type Actor%20Object%20Reference)))

(event EventTick
  (params (DeltaSeconds :type Float%20%28single-precision%29)))

(fn ConstructionScript)