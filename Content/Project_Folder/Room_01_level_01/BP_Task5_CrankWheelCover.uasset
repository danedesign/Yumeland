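; Crank wheel cover for a Room 01 puzzle that marks the task complete and fades away when its trigger component fires.
; The trigger prints a completion message, turns the button on the first BP_OverlapExample found in the world green, and sets Level04Passed.
; It also runs a one-time timeline that drives Opacity on a dynamic material, then destroys the mesh after a delay started from the timeline's update.
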(event ComponentTriggered(Comp_Trigger)
  (params (SourceInfo :type Struct%20Component%20Source%20Info%20Structure) (Name :type Name :default "None"))
  (bind _staticmesh (Variables|Default|GetStaticMesh))
  (Utilities|FlowControl|Sequence
    (:then_0
      ;[1 1 1] Get BP_OverlapExample without writing anything in level blueprint
      (bind _outactors (Actor|GetAllActorsOfClass "/Game/Testfolder/Triggerbutton/BP_OverlapExample.BP_OverlapExample_C"))
      (bind _asbp_overlap_example (Utilities|Casting|CastToBP_OverlapExample (Utilities|Array|Get(acopy) _outactors)))
      (Development|PrintString "Congratulations, you've completed Pawzzle It!")
      (Rendering|Material|SetMaterial (Variables|/Game/Testfolder/Triggerbutton/BP_OverlapExample.BP_OverlapExample_C|GetSM_Button_Base _asbp_overlap_example) 0 "/Game/AFCore/Meshes/Util/Anchor/M_Anchor_Green.M_Anchor_Green")
      (Variables|Default|SetLevel_04Passed true))
    (:then_1
      (Utilities|FlowControl|DoOnce false
        (:Completed
          (bind _returnvalue (Rendering|Material|CreateDynamicMaterialInstance _staticmesh 0 "/Game/Project_Folder/Room_01_level_01/BoxfadingManager/M_BoxfadingManager.M_BoxfadingManager" "" :!class /Script/Engine.PrimitiveComponent))
          (bind _newtrack_0 (Timeline|Timeline_0 PlayFromStart)
            (:Update
              (Rendering|Material|SetScalarParameterValue _returnvalue "Opacity" _newtrack_0 :!class /Script/Engine.MaterialInstanceDynamic)
              (Utilities|FlowControl|Delay 4.0)
              (Components|DestroyComponent _staticmesh))))))))

(event EventBeginPlay)

(event Collision|EventActorBeginOverlap
  (params (OtherActor :type Actor%20Object%20Reference)))

(fn ConstructionScript)