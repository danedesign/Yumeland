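; Window blind puzzle object for Room 01, Level 01 that fades away and is removed once its task is passed.
; An active-state change on Comp_Active sets a component's active state and flags Level3Passed.
; Component activation prints a debug message, fades the mesh through a timeline-driven dynamic material opacity, then destroys it after a delay.
; Activation also plays a 2D sound once, guarded by a DoOnce.
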(event ActiveStateChanged(Comp_Active)
  (params (SourceInfo :type Struct%20Component%20Source%20Info%20Structure) (Active :type Boolean))
  (Components|Activation|SetActive (Variables|Default|GetComp_Active) Active false)
  (Variables|Default|SetLevel%203%20Passed true))

(event OnComponentActivated(Comp_Active)
  (params (Component :type Actor%20Component%20Object%20Reference) (bReset :type Boolean))
  (bind _staticmesh (Variables|Default|GetStaticMesh))
  (Utilities|FlowControl|Sequence
    (:then_0
      (Development|PrintString "Task 5 Passed")
      (bind _returnvalue (Rendering|Material|CreateDynamicMaterialInstance _staticmesh 0 "/Game/Project_Folder/Room_01_level_01/BoxfadingManager/M_BoxfadingManager.M_BoxfadingManager" "None" :!class /Script/Engine.PrimitiveComponent))
      (bind _newtrack_0 (Timeline|Timeline_0 PlayFromStart)
        (:Update
          (Rendering|Material|SetScalarParameterValue _returnvalue "Opacity" _newtrack_0 :!class /Script/Engine.MaterialInstanceDynamic)
          (Utilities|FlowControl|Delay 4.0)
          (Components|DestroyComponent _staticmesh))))
    (:then_1
      (Utilities|FlowControl|DoOnce false
        (:Completed
          (Audio|SpawnSound2D "/Game/Project_Folder/Assets/01_Sounds/VoiceOver/Task04/Darling_if_you_could.Darling_if_you_could" 1.0 1.0 0.0 0))))))

(event EventBeginPlay)

(event Collision|EventActorBeginOverlap
  (params (OtherActor :type Actor%20Object%20Reference)))

(event EventTick
  (params (DeltaSeconds :type Float%20%28single-precision%29)))

(fn ConstructionScript)